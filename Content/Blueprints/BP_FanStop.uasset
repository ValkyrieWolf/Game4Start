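; BP_FanStop is a fan actor that spins a cylinder and has a StopFan event to halt it.
; On BeginPlay a timeline drives the cylinder's yaw and, from its update through a short delay, repeatedly binds an event to BoundSwitch's activation.
; StopFan plays a second timeline whose output is multiplied by zero, holding yaw at zero while it updates, without stopping the spin timeline.
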(event Custom|Stop%20Fan
  (bind _stop_fan (Timeline|Stop%20the%20fan PlayFromStart)
    (:Update
      (Transformation|SetRelativeRotation (Variables|Default|GetCylinder) (Math|Rotator|MakeRotator 0.0 0.0 (* _stop_fan 0.0)) false false))))

(event EventBeginPlay
  (bind _newtrack_0 (Timeline|Timeline PlayFromStart)
    (:Update
      (Transformation|SetRelativeRotation (Variables|Default|GetCylinder) (Math|Rotator|MakeRotator 0.0 0.0 (* _newtrack_0 3.6e+02)) false false)
      (if true
        (Utilities|FlowControl|Delay 0.2)
        (EventDispatchers|BindEventtoOnEventSwitchActivated (Variables|Default|GetBound%20Switch) (EventDispatchers|CreateEvent :!event Custom|Stop%20Fan))))))

(fn ConstructionScript)