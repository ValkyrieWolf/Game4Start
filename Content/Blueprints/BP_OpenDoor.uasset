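; BP_OpenDoor is a door that rises when its bound switch is activated.
; After a short delay at BeginPlay it binds an event to the BoundSwitch activation dispatcher.
; OpenDoor plays the MoveDoor timeline, lerping the static mesh upward along Z.
; Each update lerps from the mesh's current location rather than a stored start, so the offset accumulates and total travel depends on update count.
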(event Custom|Open%20Door
  (bind _staticmesh (Variables|Default|GetStaticMesh))
  (bind _returnvalue (Transformation|GetWorldLocation _staticmesh))
  (bind _alpha_track (Timeline|Move%20Door PlayFromStart)
    (:Update
      (Transformation|SetWorldLocation (Variables|Default|GetStaticMesh) (Math|Vector|Lerp(Vector) (Transformation|GetWorldLocation _staticmesh) (Math|Vector|MakeVector (.x _returnvalue) (.y _returnvalue) (+ (.z _returnvalue) 1e+01)) _alpha_track) false false))))

(event EventBeginPlay
  (Utilities|FlowControl|Delay 0.2)
  (EventDispatchers|BindEventtoOnEventSwitchActivated (Variables|Default|GetBoundSwitch) (EventDispatchers|CreateEvent :!event Custom|Open%20Door)))

(fn ConstructionScript)