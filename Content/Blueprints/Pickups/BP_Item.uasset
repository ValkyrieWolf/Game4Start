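; BP_Item is a pickup item that can be picked up, held and dropped.
; PickUp disables collision and physics on its Cube, then snaps the item to the passed skeletal mesh's right-hand item socket.
; Drop re-enables collision, detaches in world space, turns physics on and applies a fixed world-axis force to toss it.
; PrimaryAction is a placeholder that only prints a debug message.
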(event Custom|PickUp
  (params (Skeletal%20Mesh :type Scene%20Component%20Object%20Reference))
  (Development|PrintString "Calling Pick Up!" true true "(R=0.778321,G=1.000000,B=0.000000,A=1.000000)" 4.0)
  (Collision|SetCollisionEnabled (Variables|Default|GetCube) "NoCollision") ; don't push us off map
  (Physics|SetSimulatePhysics (Variables|Default|GetCube) false)
  (Transformation|AttachComponentToComponent Skeletal%20Mesh "item_socket_r" "SnapToTarget" "SnapToTarget" "KeepRelative" true) ; Attaches the item to the player's socket
)

(event Custom|Drop
  (Development|PrintString "Dropping Item!")
  (Collision|SetCollisionEnabled (Variables|Default|GetCube) "QueryAndPhysics")
  (Transformation|DetachFromActor "KeepWorld" "KeepWorld" "KeepRelative")
  (Physics|SetSimulatePhysics (Variables|Default|GetCube) true)
  (Physics|AddForce (Variables|Default|GetCube) "500.000000,0.000000,200.000000" "" false))

(event Custom|PrimaryAction
  (Development|PrintString "Testing Primary Action!"))

(fn ConstructionScript)