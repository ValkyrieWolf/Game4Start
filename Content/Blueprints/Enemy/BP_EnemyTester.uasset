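; BP_EnemyTester is a test actor that repeatedly damages every BP_Enemy in the level.
; On BeginPlay it gathers all BP_Enemy actors, prints their count, and calls TakeDamage on each with a small random amount, printing each array index.
; After a two-second delay it calls the GiveDamage event, which wires back to the search, so the cycle repeats indefinitely.
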(event Custom|GiveDamage
  (bind _outactors (Actor|GetAllActorsOfClass "/Game/Blueprints/Enemy/BP_Enemy.BP_Enemy_C")) ; Fin all of the BP_Enemy Class
  (Development|PrintString (Utilities|String|Append "There are: " (Utilities|String|ToString(Integer) (Utilities|Array|Length _outactors)) " enemies in the level!"))
  (for (_array_element _array_index) _outactors
    (Default|TakeDamage _array_element (Math|Random|RandomFloatinRange 0.1 0.5))
    (Development|PrintString (Utilities|String|Append "Array Index = " (Utilities|String|ToString(Integer) _array_index)) true true "(R=0.000000,G=0.660000,B=1.000000,A=1.000000)" 3.5))
  (Development|PrintString "We've given damage to all of the enemies!" true true "(R=0.413284,G=1.000000,B=0.887844,A=1.000000)" 5.0)
  (Utilities|FlowControl|Delay 2.0)
  (CallFunction|GiveDamage))

(event EventBeginPlay
  (bind _outactors (Actor|GetAllActorsOfClass "/Game/Blueprints/Enemy/BP_Enemy.BP_Enemy_C")) ; Fin all of the BP_Enemy Class
  (Development|PrintString (Utilities|String|Append "There are: " (Utilities|String|ToString(Integer) (Utilities|Array|Length _outactors)) " enemies in the level!"))
  (for (_array_element _array_index) _outactors
    (Default|TakeDamage _array_element (Math|Random|RandomFloatinRange 0.1 0.5))
    (Development|PrintString (Utilities|String|Append "Array Index = " (Utilities|String|ToString(Integer) _array_index)) true true "(R=0.000000,G=0.660000,B=1.000000,A=1.000000)" 3.5))
  (Development|PrintString "We've given damage to all of the enemies!" true true "(R=0.413284,G=1.000000,B=0.887844,A=1.000000)" 5.0)
  (Utilities|FlowControl|Delay 2.0)
  (CallFunction|GiveDamage))

(event Collision|EventActorBeginOverlap
  (params (OtherActor :type Actor%20Object%20Reference)))

(event EventTick
  (params (DeltaSeconds :type Float%20%28single-precision%29)))

(fn ConstructionScript)