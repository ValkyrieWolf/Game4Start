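; BP_Enemy is a basic enemy Blueprint that announces itself with a red on-screen message on BeginPlay.
; Its TakeDamage event prints a pain message, subtracts the incoming amount from Health, then destroys the actor when CheckIfDead finds Health at or below zero.
; Overlap, Tick and the construction script are empty, and the graphs contain no movement or attack logic.
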(event Custom|TakeDamage
  (params (By%20Amount :type Float%20%28double-precision%29))
  (Development|PrintString "Ouch!" true true "(R=1.000000,G=0.000000,B=0.032468,A=1.000000)" 3.5)
  (bind _output_get (Variables|Default|SetHealth (- (Variables|Default|GetHealth) By%20Amount)))
  (if (CallFunction|CheckifDead _output_get)
    (Actor|DestroyActor)))

(event EventBeginPlay
  (Development|PrintString "Hello I have been progammed to destroy you!" true true "(R=1.000000,G=0.112509,B=0.000000,A=1.000000)" 5.0))

(event Collision|EventActorBeginOverlap
  (params (OtherActor :type Actor%20Object%20Reference)))

(event EventTick
  (params (DeltaSeconds :type Float%20%28single-precision%29)))

(fn ConstructionScript)

(fn CheckifDead
  (params (Health :type Float%20%28double-precision%29))
  (return (<= Health 0.0)))